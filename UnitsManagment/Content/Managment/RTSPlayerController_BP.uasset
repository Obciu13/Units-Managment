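; RTS player controller that pans the camera pawn and handles unit selection and orders.
; Left click clears the selection and picks the unit under the cursor; holding it signals the HUD for multi-selection while disabling attack range colliders.
; Right click sends all selected units to the cursor hit location with AI Move To.
; Separate axis inputs directly move the main unit, taken from the first selected.
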(event `InputAxis|MoveCameraUp`
  (params (AxisValue :type "Float (single-precision)"))
  ;[1 1 1] Moving Camera pawn
  (`RTSPlayerSpectatorPawn.MoveUp` (`self.CameraPawn`) AxisValue))

(event `Key|LeftMouseButton`
  (params (Key :type "Key Structure"))
  ;[1 1 1] On Left Mouse Button Clicked
  ;;[1 1 1] Selecting Single Unit
  (:`Pressed`
    (`self.Clear Selected`)
    (bind _asunit_base_bp (cast `/Game/Units/UnitBase_BP` (`.HitActor` (`GameplayStatics.BreakHitResult` (`self.GetHitResultUnderCursorByChannel` "TraceTypeQuery2")))))
    (`/Game/Units/UnitBase_BP.OnClickedUnit` _asunit_base_bp)
    (`KismetArrayLibrary.Array_AddUnique` (`self.Selected Units`) _asunit_base_bp)
    (`self.Select Main Unit`)))

(event `InputAxis|MoveCameraRight`
  (params (AxisValue :type "Float (single-precision)"))
  ;[1 1 1] Moving Camera pawn
  (`RTSPlayerSpectatorPawn.MoveRight` (`self.CameraPawn`) AxisValue))

(event `InputAxis|MoveUnitUp`
  (params (AxisValue :type "Float (single-precision)"))
  ;[1 1 1] Moving for first selected unit
  (if (`KismetSystemLibrary.IsValid` (`self.Selected Unit`))
    (`UnitBase.MoveUp` (`self.Selected Unit`) AxisValue)))

(event `InputAxis|MoveUnitRight`
  (params (AxisValue :type "Float (single-precision)"))
  ;[1 1 1] Moving for first selected unit
  (if (`KismetSystemLibrary.IsValid` (`self.Selected Unit`))
    (`UnitBase.MoveRight` (`self.Selected Unit`) AxisValue)))

(event `Key|LeftMouseButton`
  (params (Key :type "Key Structure"))
  (bind _returnvalue (`self.GetHUD`))
  ;[1 1 1] On Left Mouse Button Clicked
  ;;[1 1 1] Selecting Multiple Units
  (:`Pressed`
    (message `/Game/Managment/SelectionInterface.StartSelection` _returnvalue)
    (`self.DisableAttackRangeColilders`))
  (:`Released`
    (message `/Game/Managment/SelectionInterface.StopSelection` _returnvalue)
    (`self.EnableAttackRangeColilders`)))

(event `Key|RightMouseButton`
  (params (Key :type "Key Structure"))
  ;[1 1 1] Move Selected Units
  (:`Pressed`
    (for _array_element (`self.Selected Units`)
      (`|AIMoveTo` _array_element (`.Location` (`GameplayStatics.BreakHitResult` (`self.GetHitResultUnderCursorByChannel` "TraceTypeQuery2"))) null))))

(fn `Clear Selected`
  (bind _selected_units (`self.Selected Units`))
  (for _array_element _selected_units
    (bind _asunit_base_bp (cast `/Game/Units/UnitBase_BP` _array_element))
    (`/Game/Units/UnitBase_BP.UnSelect` _asunit_base_bp))
  (`KismetArrayLibrary.Array_Clear` _selected_units))

(fn `Select Main Unit`
  (bind _selected_units (`self.Selected Units`))
  (if (> (`KismetArrayLibrary.Array_Length` _selected_units) 0)
    (set `self.Selected Unit` (`|GetArrayItem` _selected_units))))

(fn `UserConstructionScript`)