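; UnitBase_BP is a base Blueprint for selectable RTS units.
; Clicking a unit toggles its IsSelected flag through Select and UnSelect, which swap the mesh material to show selection state.
; It caches the RTS player controller on BeginPlay and removes itself from that controller's SelectedUnits list before destruction.
; Select and UnSelect only change local state and visuals, leaving the controller's list untouched.
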(event `self.ReceiveBeginPlay`
  ;[1 1 1] Begin Play
  (`parent.ReceiveBeginPlay`)
  (bind _asrtsplayer_controller_bp (cast `/Game/Managment/RTSPlayerController_BP` (`GameplayStatics.GetPlayerController` 0)))
  (set `self.Player Controller` _asrtsplayer_controller_bp))

(event `OnClickedUnit`
  ;[1 1 1] Select Unit on Clicked
  (if (`self.IsSelected`)
    (`self.UnSelect`)
    (else
      (`self.Select`))))

(event `self.DestroyUnit`
  ;[1 1 1] Event Destroy Unit
  (`KismetArrayLibrary.Array_RemoveItem` (`/Game/Managment/RTSPlayerController_BP.Selected Units` (`self.Player Controller`)) self)
  (`self.K2_DestroyActor`))

(fn `Select`
  (set `self.IsSelected` true)
  (`PrimitiveComponent.SetMaterial` (`self.UnitMesh`) 0 "/Engine/EngineDebugMaterials/VertexColorViewMode_GreenOnly.VertexColorViewMode_GreenOnly"))

(fn `UnSelect`
  (set `self.IsSelected` false)
  (`PrimitiveComponent.SetMaterial` (`self.UnitMesh`) 0 "/Engine/BufferVisualization/WorldNormal.WorldNormal"))

(fn `UserConstructionScript`)